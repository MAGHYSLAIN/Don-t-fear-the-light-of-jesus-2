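; Enemy actor that takes the form of a Wi-Fi icon, ice cream cone or clock and is destroyed by bullets.
; The construction script picks the mesh and material of the Sphere component from NMEEnum.
; A Bullet overlapping the Box spawns a scaled-up explosion at the Sphere's location and destroys the actor.
; SetMeshFunction repeats the same mesh switch for a passed-in selection but is not called within this Blueprint.
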(event `self.Box.OnComponentBeginOverlap`
  (params (OverlappedComponent :type "PrimitiveComponent Object Reference") (OtherActor :type "Actor Object Reference") (OtherComp :type "PrimitiveComponent Object Reference") (OtherBodyIndex :type Integer) (bFromSweep :type Boolean) (SweepResult :type "HitResult Structure (by ref)"))
  (cast `/Game/Characters/ProtoVulture/Bullet` OtherActor)
  (`GameplayStatics.SpawnEmitterAtLocation` "/Game/StarterContent/Particles/P_Explosion.P_Explosion" (`SceneComponent.K2_GetComponentLocation` (`self.Sphere`)) (struct) (10.0 10.0 10.0))
  (`self.K2_DestroyActor`))

(fn `SetMeshFunction`
  (params (Selection :type "/Game/Blueprint/NME_Enum Enum" :default "NewEnumerator0"))
  (bind _sphere (`self.Sphere`))
  (bind _sphere_2 (`self.Sphere`))
  (bind _sphere_3 (`self.Sphere`))
  (switch `/Game/Blueprint/NME_Enum` Selection
    (:`NewEnumerator0`
      (`StaticMeshComponent.SetStaticMesh` _sphere_2 "/Game/Assets/WIFI/Meshy_AI_Glossy_Wi_Fi_Icon_0817022014_texture.Meshy_AI_Glossy_Wi_Fi_Icon_0817022014_texture")
      (`PrimitiveComponent.SetMaterial` _sphere_2 0 "/Game/Assets/WIFI/Material_001.Material_001"))
    (:`NewEnumerator1`
      (`StaticMeshComponent.SetStaticMesh` _sphere_3 "/Game/Assets/IceCream/Meshy_AI_Lime_Cream_Cone_0821031519_texture.Meshy_AI_Lime_Cream_Cone_0821031519_texture")
      (`PrimitiveComponent.SetMaterial` _sphere_3 0 "/Game/Assets/IceCream/Material_001.Material_001"))
    (:`NewEnumerator2`
      (`StaticMeshComponent.SetStaticMesh` _sphere "/Game/Assets/Clock/Meshy_AI_Golden_Clock_on_Green_0821031751_texture.Meshy_AI_Golden_Clock_on_Green_0821031751_texture")
      (`PrimitiveComponent.SetMaterial` _sphere 0 "/Game/Assets/Clock/Material_001.Material_001"))))

(fn `UserConstructionScript`
  (bind _sphere (`self.Sphere`))
  (bind _sphere_2 (`self.Sphere`))
  (bind _sphere_3 (`self.Sphere`))
  (switch `/Game/Blueprint/NME_Enum` (`self.NME_Enum`)
    (:`NewEnumerator0`
      (`StaticMeshComponent.SetStaticMesh` _sphere_2 "/Game/Assets/WIFI/Meshy_AI_Glossy_Wi_Fi_Icon_0817022014_texture.Meshy_AI_Glossy_Wi_Fi_Icon_0817022014_texture")
      (`PrimitiveComponent.SetMaterial` _sphere_2 0 "/Game/Assets/WIFI/Material_001.Material_001"))
    (:`NewEnumerator1`
      (`StaticMeshComponent.SetStaticMesh` _sphere_3 "/Game/Assets/IceCream/Meshy_AI_Lime_Cream_Cone_0821031519_texture.Meshy_AI_Lime_Cream_Cone_0821031519_texture")
      (`PrimitiveComponent.SetMaterial` _sphere_3 0 "/Game/Assets/IceCream/Material_001.Material_001"))
    (:`NewEnumerator2`
      (`StaticMeshComponent.SetStaticMesh` _sphere "/Game/Assets/Clock/Meshy_AI_Golden_Clock_on_Green_0821031751_texture.Meshy_AI_Golden_Clock_on_Green_0821031751_texture")
      (`PrimitiveComponent.SetMaterial` _sphere 0 "/Game/Assets/Clock/Material_001.Material_001"))))