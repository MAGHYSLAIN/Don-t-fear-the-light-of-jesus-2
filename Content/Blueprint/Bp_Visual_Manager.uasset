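; Visual manager actor that toggles screen effects on a Chameleon actor from debug-style number key presses.
; On BeginPlay it caches the first Chameleon found in the level.
; Keys 1, 2 and 3 each drive a FlipFlop that switches the Mosaic, Drug or Alcohol flag on and off.
; Each toggle also calls ActivateEffect or DesactivateEffect, both of which are empty stubs.
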(event `self.ReceiveBeginPlay`
  (bind _outactors (`GameplayStatics.GetAllActorsOfClass` "/Game/Chameleon/Chameleon.Chameleon_C"))
  (set `self.Chameleon` (`|GetArrayItem` _outactors)))

(event `Key|One` :consume false :overrideparent false
  (params (Key :type "Key Structure"))
  (bind _chameleon (`self.Chameleon`))
  (:`Pressed`
    ;[1 1 1] Mosaic
    (`/Engine/EditorBlueprintResources/StandardMacros.FlipFlop`
      (:`A`
        (`self.ActivateEffect`)
        (set `/Game/Chameleon/Chameleon.Mosaic` true _chameleon))
      (:`B`
        (`self.DesactivateEffect`)
        (set `/Game/Chameleon/Chameleon.Mosaic` false _chameleon)))))

(event `Key|Two`
  (params (Key :type "Key Structure"))
  (bind _chameleon (`self.Chameleon`))
  (:`Pressed`
    ;[1 1 1] Template
    (`/Engine/EditorBlueprintResources/StandardMacros.FlipFlop`
      (:`A`
        (`self.ActivateEffect`)
        (set `/Game/Chameleon/Chameleon.Drug` true _chameleon))
      (:`B`
        (`self.DesactivateEffect`)
        (set `/Game/Chameleon/Chameleon.Drug` false _chameleon)))))

(event `Key|Three`
  (params (Key :type "Key Structure"))
  (bind _chameleon (`self.Chameleon`))
  (:`Pressed`
    ;[1 1 1] Template
    (`/Engine/EditorBlueprintResources/StandardMacros.FlipFlop`
      (:`A`
        (`self.ActivateEffect`)
        (set `/Game/Chameleon/Chameleon.Alcohol` true _chameleon))
      (:`B`
        (`self.DesactivateEffect`)
        (set `/Game/Chameleon/Chameleon.Alcohol` false _chameleon)))))

(event `Key|Four`
  (params (Key :type "Key Structure")))

(event `Key|Six`
  (params (Key :type "Key Structure")))

(event `Key|Five`
  (params (Key :type "Key Structure")))

(event `Key|Seven`
  (params (Key :type "Key Structure")))

(fn `ActivateEffect`)

(fn `DesactivateEffect`)

(fn `UserConstructionScript`)